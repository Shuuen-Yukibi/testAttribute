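; Stamina component that handles sprinting, one-off stamina costs and regeneration for its owning actor.
; Sprint input switches walk speed and starts a looping timer that drains stamina while moving, stopping when empty.
; Stopping or spending stamina triggers regeneration through a retriggerable delay, which resumes the timer only if not sprinting.
; Stamina changes are clamped to the maximum and broadcast as a fraction through the OnStaminaChanged dispatcher.
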(event `EnhancedInput|/Game/CoreSystems/DemoContent/ThirdPerson/Input/Actions/IA_Sprint`
  (params (ActionValue :type Boolean) (ElapsedSeconds :type "Float (double-precision)") (TriggeredSeconds :type "Float (double-precision)") (InputAction :type "InputAction Object Reference" :default "/Game/CoreSystems/DemoContent/ThirdPerson/Input/Actions/IA_Sprint.IA_Sprint"))
  ;[1 1 1] Sprint Input action this could be on the player if needs be
  (:`Triggered`
    ;[1 1 1] only need set stuff once no point going through nodes past here after initial hold
    (`/Engine/EditorBlueprintResources/StandardMacros.DoOnce` false :!label _label
      (:`Completed`
        ;[1 1 1] Starts the sprinting function
        (`self.StartSprinting`))))
  (:`Completed`
    ;[1 1 1] On release of key stops sprinting function and reset node to enable sprinting again
    (`self.StopSprinting`)
    (goto _label :!via `Reset`)))

(event `ModifyStaminaEvenet`
  (params (ModifyAmount :type "Float (double-precision)") (increase :type Boolean))
  ;[1 1 1] Starts a loop to modify the stamina every 0.1 second until loop is stopped use a retrigg delay to keep reseting the regen if stop start sprinting, if hit delay and then start sprinting branch will catch so regen and degen dont happen at same time
  (if increase
    (`KismetSystemLibrary.RetriggerableDelay` 5.0)
    (if (not (`self.Sprinting`))
      (bind _returnvalue (`KismetSystemLibrary.K2_SetTimerDelegate` (delegate `ModifyLoop`) 0.1 true :!label _label_2))
      (set `self.LoopTimer` _returnvalue))
    (else
      (goto _label_2))))

(event `ModifyLoop`
  (`self.StaminaChange` (stale `ModifyStaminaEvenet` ModifyAmount) (stale `ModifyStaminaEvenet` increase)))

(fn `CalculateStaminaPercentages`
  ;[1 1 1] Calculates percentages and tells any one listening via dispatcher that stamina has changed.
  (`self.OnStaminaChanged` (`KismetMathLibrary.SafeDivide` (`self.CurrentStamina`) (`self.MaxStamina`))))

(fn `IncreaseMaxStamina`
  (params (IncreasemaxStaminaBy :type "Float (double-precision)"))
  ;[1 1 1] IncreaseMax stamina and then recalculates values
  (set `self.MaxStamina` (+ (`self.MaxStamina`) IncreasemaxStaminaBy))
  (`self.CalculateStaminaPercentages`))

(fn `SetStartingStaminaValues`
  (`self.IncreaseMaxStamina` 0.0)
  (`self.CalculateStaminaPercentages`)
  (`self.ModifyStaminaEvenet` (`self.StaminaRegenRate`) true))

(fn `StaminaChange`
  (params (Value :type "Float (double-precision)") (Increase :type Boolean))
  (if (`self.Sprinting`)
    ;[1 1 1] Checks if player is stood still if stood still we dont want to stop increasing stamina or decrease it all
    (if (> (`KismetMathLibrary.VSize` (`Actor.GetVelocity` (`self.GetOwner`))) 0.0)
      ;[1 1 1] Sets new stamina value
      (bind _output_get (set `self.CurrentStamina` (`KismetMathLibrary.FClamp` (- (`self.CurrentStamina`) (select `bool` (`local.Increase`) :`false` (`local.Value`) :`true` (* (`local.Value`) -1.0))) 0.0 (`self.MaxStamina`)) :!label _label))
      ;[1 1 1] Calls the calculate function to change percentages
      (`self.CalculateStaminaPercentages`)
      ;[1 1 1] if stamina not empty continue if empty stop sprinting
      (if (or (<= _output_get 0.0) (>= _output_get (`self.MaxStamina`)))
        (`self.StopSprinting`)))
    (else
      (goto _label))))

(fn `StartSprinting`
  (bind _returnvalue (`Actor.GetComponentByClass` (`self.GetOwner`) "/Script/Engine.CharacterMovementComponent"))
  ;[1 1 1] Starts sprinting and sets speed to higher
  (set `self.Sprinting` true)
  (`/Engine/EditorBlueprintResources/StandardMacros.IsValid` _returnvalue
    (:`Is Valid`
      (set `CharacterMovementComponent.MaxWalkSpeed` 800.0 _returnvalue))
    (:`Is Not Valid`
      _))
  ;[1 1 1] starts a degeneration event
  (`self.ModifyStaminaEvenet` 1.0))

(fn `StopSprinting`
  (bind _returnvalue (`Actor.GetComponentByClass` (`self.GetOwner`) "/Script/Engine.CharacterMovementComponent"))
  ;[1 1 1] Stop the loop and reset stamina if dont ahve the movement component but does have stamina such as flying boss etc then continue and start regenration event
  (set `self.Sprinting` false)
  (`KismetSystemLibrary.K2_ClearAndInvalidateTimerHandle` (`self.LoopTimer`))
  (`/Engine/EditorBlueprintResources/StandardMacros.IsValid` _returnvalue
    (:`Is Valid`
      (set `CharacterMovementComponent.MaxWalkSpeed` 500.0 _returnvalue))
    (:`Is Not Valid`
      _))
  ;[1 1 1] The tick to increase starts regenaration
  (`self.ModifyStaminaEvenet` (`self.StaminaRegenRate`) true))

(fn `Use Stamina`
  (params (Value :type "Float (double-precision)"))
  (returns (EnoughStamina :type Boolean))
  ;[1 1 1] If not enough curent stamina then exit function if enough continue
  (if (>= (`self.CurrentStamina`) (`local.Value`))
    ;[1 1 1] Change the stamina and then call the regeneration event
    (`self.StaminaChange` (`local.Value`))
    (`self.ModifyStaminaEvenet` (`self.StaminaRegenRate`) true)
    (return true)
    (else
      (return false))))
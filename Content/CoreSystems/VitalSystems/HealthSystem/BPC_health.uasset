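; Reusable health component that tracks current and max health, broadcasting percentage changes and death for other code to handle.
; Clamped increase and decrease functions drive looping timers for regeneration and damage over time.
; Non-lethal damage restarts regeneration through a retriggerable delay.
; Healing cancels damage over time and damage cancels regeneration, so the two loops do not run together.
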(event `RegenHealth`
  (params (RegenRate :type "Float (double-precision)"))
  ;[1 1 1] controls how long before mana starts regening
  (`KismetSystemLibrary.RetriggerableDelay` 2.0)
  (if (not (<= (`self.CurrentHealth`) 0.0))
    ;[1 1 1] reduces every 0.1 second
    (bind _returnvalue (`KismetSystemLibrary.K2_SetTimerDelegate` (delegate `RegenLoop`) 0.1 true))
    (set `self.RegenTimer` _returnvalue)))

(event `RegenLoop`
  ;[1 1 1] Increase by the regen rate for mana
  (bind _healthfull (`self.IncreaseHealth` (stale `RegenHealth` RegenRate)))
  (if _healthfull
    (`self.StopRegenTimer`)))

(event `DamageOverTime`
  (params (AmountToDecreaseBy :type "Float (double-precision)"))
  (`self.StopRegenTimer`)
  ;[1 1 1] reduces every 0.1 second
  (bind _returnvalue (`KismetSystemLibrary.K2_SetTimerDelegate` (delegate `DOTLoop`) 0.1 true))
  (set `self.DOTTimer` _returnvalue))

(event `DOTLoop`
  ;[1 1 1] Increase by the regen rate for mana
  (bind _dead (`self.DecreaseHealth` (stale `DamageOverTime` AmountToDecreaseBy)))
  (if _dead
    (`self.StopDOTTimer`)))

(fn `CalculateHealthPercentage`
  ;[1 1 1] Calculate ths mana percentage
  (`self.OnHealthChanged` (`KismetMathLibrary.SafeDivide` (`self.CurrentHealth`) (`self.MaxHealth`))))

(fn `DecreaseHealth`
  (params (AmountToDecreaseBy :type "Float (double-precision)"))
  (returns (Dead :type Boolean))
  ;[1 1 1] cancels the regen timer so not regening and decreasing ats ame time
  (`self.StopRegenTimer`)
  ;[1 1 1] Gets health and reduces the amount and calculates the percentage for the UI
  (bind _output_get (set `self.CurrentHealth` (`KismetMathLibrary.FClamp` (- (`self.CurrentHealth`) (`local.AmountToDecreaseBy`)) 0.0 (`self.MaxHealth`))))
  (`self.CalculateHealthPercentage`)
  (if (<= _output_get 0.0)
    ;[1 1 1] Calls the dead event to be handled seperatley could also be handled here as well but this component can be used for physical objects and characters implementing ragdoll in here wouldnt work for both for eaxample
    (`self.StopRegenTimer`)
    (`self.OnDead`)
    (return true)
    (else
      ;[1 1 1] Calls the regen event which will hit the retrigable delay if on the loop
      (`self.RegenHealth` (`self.HealthRegenRate`))
      (return false))))

(fn `IncreaseHealth`
  (params (IncreasAmount :type "Float (double-precision)"))
  (returns (HealthFull :type Boolean))
  ;[1 1 1] Increases health stops going above max
  (`self.StopDOTTimer`)
  (bind _output_get (set `self.CurrentHealth` (`KismetMathLibrary.FClamp` (+ (`self.CurrentHealth`) IncreasAmount) 0.0 (`self.MaxHealth`))))
  (`self.CalculateHealthPercentage`)
  (if (>= _output_get (`self.MaxHealth`))
    (return true)
    (else
      (return false))))

(fn `IncreaseMaxHealth`
  (params (IncreasemaxManaBy :type "Float (double-precision)"))
  ;[1 1 1] Increase Max mana and re calcualte percentages
  (set `self.MaxHealth` (+ (`self.MaxHealth`) IncreasemaxManaBy))
  (`self.CalculateHealthPercentage`))

(fn `SetHealthStartingValues`
  ;[1 1 1] Sets the starting values for health
  (`self.IncreaseMaxHealth` 0.0)
  (`self.CalculateHealthPercentage`)
  (`self.RegenHealth` (`self.HealthRegenRate`)))

(fn `StopDOTTimer`
  ;[1 1 1] Stops the damage over time timer
  (`KismetSystemLibrary.K2_ClearAndInvalidateTimerHandle` (`self.DOTTimer`)))

(fn `StopRegenTimer`
  ;[1 1 1] Stops regen timer cleaner here for use in owners bps
  (`KismetSystemLibrary.K2_ClearAndInvalidateTimerHandle` (`self.RegenTimer`)))